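; BP_VoluCloudEdit is a volumetric cloud painting tool that writes spherical density brushes into a render target.
; UpdateTraces projects a point along the actor's forward vector, draws debug guides colored by whether it lies in the target mesh's box, and stores it in local space.
; PaintVolume draws a dynamic painter material fed with brush center, density and scale-adjusted radius onto the canvas, and ResetRT clears it.
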(event EventBeginPlay
  (bind _returnvalue (Rendering|Material|CreateDynamicMaterialInstance "/Game/_hamagami/RMCS/Assets/M_vol_painter.M_vol_painter" "None" "None" :!class /Script/Engine.KismetMaterialLibrary))
  (Variables|Default|SetDMI_vol_painter _returnvalue))

(event EventTick
  (params (DeltaSeconds :type Float%20%28single-precision%29)))

(fn ConstructionScript)

(fn PaintVolume
  (bind _dmi_vol_painter (Variables|Default|GetDMI_vol_painter))
  (bind (_canvas _size _context) (Rendering|BeginDrawCanvastoRenderTarget (Variables|Default|GetRT)))
  (Rendering|Material|SetVectorParameterValue _dmi_vol_painter "SphereCenter" (Math|Conversions|ToLinearColor(Vector) (Variables|Default|GetPaintPosition)) :!class /Script/Engine.MaterialInstanceDynamic)
  (Rendering|Material|SetScalarParameterValue _dmi_vol_painter "Density" (Variables|Default|GetPaintDensity) :!class /Script/Engine.MaterialInstanceDynamic)
  (Rendering|Material|SetScalarParameterValue _dmi_vol_painter "Radius" (/ (Variables|Default|GetPaintRadius) (.X (Math|Vector|BreakVector (Transformation|GetActorScale3D (Variables|Default|GetTargetSphereMesh))))) :!class /Script/Engine.MaterialInstanceDynamic)
  (Canvas|DrawMaterial :self _canvas :RenderMaterial _dmi_vol_painter :ScreenSize _size :CoordinateSize "(X=1.000000,Y=1.000000)" :PivotPoint "(X=0.500000,Y=0.500000)")
  (Rendering|EndDrawCanvastoRenderTarget _context))

(fn ResetRT
  (Rendering|ClearRenderTarget2D (Variables|Default|GetRT)))

(fn UpdateTraces
  (bind _returnvalue (Transformation|GetActorLocation))
  (bind _returnvalue_2 (Transformation|GetActorForwardVector))
  (bind _targetspheremesh (Variables|Default|GetTargetSphereMesh))
  (bind _tracedistance (Variables|Default|GetTraceDistance))
  (bind _paintradius (Variables|Default|GetPaintRadius))
  (bind _returnvalue_3 (Transformation|GetActorLocation _targetspheremesh))
  (bind _returnvalue_4 (Transformation|GetActorScale3D _targetspheremesh))
  (bind _returnvalue_5 (* _returnvalue_2 _tracedistance))
  (bind _returnvalue_6 (* _paintradius 5e+01))
  (bind _returnvalue_7 (* _returnvalue_4 5e+01))
  (bind _returnvalue_8 (+ _returnvalue _returnvalue_5))
  (if (Variables|Default|GetShowGuids)
    (Rendering|Debug|DrawDebugBox _returnvalue_3 _returnvalue_7 "(R=1.000000,G=0.000000,B=0.000000,A=1.000000)" (Transformation|GetActorRotation _targetspheremesh) 0.0 0.0)
    (bind _output_get (Variables|Default|SetValiPaintPosition (Class|KismetMathLibrary|BoxIsPointInside (Class|KismetMathLibrary|MakeBoxwithOrigin _returnvalue_3 _returnvalue_7) _returnvalue_8)))
    (if _output_get
      (Rendering|Debug|DrawDebugSphere _returnvalue_8 _returnvalue_6 12 "(R=0.000000,G=1.000000,B=0.000000,A=1.000000)" 0.0)
      (Variables|Default|SetPaintPosition (/ (Math|Transform|InverseTransformLocation (Transformation|GetActorTransform _targetspheremesh) _returnvalue_8) 5e+01))
      (else
        (Rendering|Debug|DrawDebugSphere _returnvalue_8 _returnvalue_6 12 "(R=1.000000,G=0.000000,B=0.000000,A=1.000000)" 0.0)))))

(fn GetFloat
  (return (Variables|Default|GetPaintRadius) (Variables|Default|GetPaintDensity)))