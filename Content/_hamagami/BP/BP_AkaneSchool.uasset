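; BP_AkaneSchool is the Akane character actor, with events for animations and for revealing her other figure.
; BeginPlay hides the capsule and its children, and Tick keeps the Akane component's visibility synced to OtherVisible.
; VisibleOtherFigure sets that flag and runs a timeline driving the "Amount" material parameter on Akane.
; Status1 plays a one-shot animation on Mesh, and Story1 plays another on both Mesh and Akane.
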(event Custom|Status1
  (Components|Animation|PlayAnimation (Variables|Character|GetMesh) "/Game/_nishimiya/Akane_face/Akane_Animation001_face.Akane_Animation001_face" false))

(event Custom|Story1
  (Components|Animation|PlayAnimation (Variables|Character|GetMesh) "/Game/_nishimiya/Akane_face/Akane_Animation005_face.Akane_Animation005_face" false))

(event Custom|VisibleOtherFigure
  (Variables|Default|SetOtherVisible true)
  (bind _新規track_0 (Timeline|タイムライン PlayFromStart)
    (:Update
      (Rendering|Material|SetScalarParameterValueonMaterials (Variables|Default|GetAkane) "Amount" _新規track_0))))

(event EventBeginPlay
  (Rendering|SetVisibility (Variables|Collision|GetCapsuleComponent) false true))

(event Collision|EventActorBeginOverlap
  (params (OtherActor :type Actor%20Object%20Reference)))

(event EventTick
  (params (DeltaSeconds :type Float%20%28single-precision%29))
  (Rendering|SetVisibility (Variables|Default|GetAkane) (Variables|Default|GetOtherVisible) false))

(fn ConstructionScript)