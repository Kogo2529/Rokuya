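; Component that drives a tackle aura on its owning actor using two Niagara effects, a meteor aura and a fire trail.
; BeginPlay spawns both systems unattached, sets their ScaleAlpha and passes Distance to the aura as Length.
; Tick updates ScaleAlpha and rebinds the trail to TargetMesh.
; While ScaleAlpha is above zero, it moves the aura to the owner with location and rotation offsets, and the trail to the mesh.
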(event EventBeginPlay
  (bind _returnvalue (Components|GetOwner))
  (bind _rotation (Variables|Default|GetRotation))
  (bind _returnvalue_2 (Transformation|GetActorRotation _returnvalue))
  (bind (_roll _pitch _yaw) (Math|Rotator|BreakRotator _rotation))
  (Utilities|FlowControl|Sequence
    (:then_0
      (bind _returnvalue_3 (Niagara|SpawnSystematLocation "/Game/_hamagami/VFX/NS/NS_FireTrail.NS_FireTrail" (Transformation|GetActorLocation (Components|GetOwner)) "0, 0, 0" "1.000000,1.000000,1.000000" false))
      (if (Utilities|IsValid _returnvalue_3)
        (bind _output_get (Variables|Default|SetTrail _returnvalue_3))
        (Niagara|SetNiagaraVariable(Float) _output_get "ScaleAlpha" (Variables|Default|GetScaleAlpha))
        (else
          (Development|PrintString "Hello" true true "(R=0.000000,G=0.660000,B=1.000000,A=1.000000)" 5.0))))
    (:then_1
      (bind _returnvalue_4 (Niagara|SpawnSystematLocation "/Game/_hamagami/VFX/NS/NS_MeteorAura.NS_MeteorAura" (+ (Transformation|GetActorLocation (Components|GetOwner)) (Variables|Default|GetLocalLocation)) (Math|Rotator|MakeRotator (+ (.roll _returnvalue_2) _roll) (+ (.pitch _returnvalue_2) _pitch) (+ (.yaw _returnvalue_2) _yaw)) (Variables|Default|GetScale) false))
      (bind _output_get_2 (Variables|Default|SetVFX _returnvalue_4))
      (Niagara|SetNiagaraVariable(Float) _output_get_2 "ScaleAlpha" (Variables|Default|GetScaleAlpha))
      (Niagara|SetNiagaraVariable(Float) _output_get_2 "Length" (Variables|Default|GetDistance)))))

(event EventTick
  (params (DeltaSeconds :type Float%20%28single-precision%29))
  (bind _returnvalue (Components|GetOwner))
  (bind _scalealpha (Variables|Default|GetScaleAlpha))
  (bind _rotation (Variables|Default|GetRotation))
  (bind (_roll _pitch _yaw) (Math|Rotator|BreakRotator _rotation))
  (bind _returnvalue_2 (Transformation|GetActorRotation _returnvalue))
  (Class|NiagaraFunctionLibrary|OverrideSystemUserVariableSkeletalMeshComponent (Variables|Default|GetTrail) "" (Variables|Default|GetTargetMesh))
  (Niagara|SetNiagaraVariable(Float) (Variables|Default|GetVFX) "ScaleAlpha" _scalealpha)
  (Niagara|SetNiagaraVariable(Float) (Variables|Default|GetTrail) "ScaleAlpha" _scalealpha)
  (if (not (<= (Variables|Default|GetScaleAlpha) 0.0))
    (Transformation|SetWorldLocation (Variables|Default|GetVFX) (+ (Transformation|GetActorLocation (Components|GetOwner)) (Variables|Default|GetLocalLocation)) false false)
    (Transformation|SetWorldRotation (Variables|Default|GetVFX) (Math|Rotator|MakeRotator (+ (.roll _returnvalue_2) _roll) (+ (.pitch _returnvalue_2) _pitch) (+ (.yaw _returnvalue_2) _yaw)) false false)
    (Transformation|SetWorldLocation (Variables|Default|GetTrail) (Transformation|GetWorldLocation (Variables|Default|GetTargetMesh)) false false)
    (Transformation|SetWorldRotation (Variables|Default|GetTrail) (Transformation|GetWorldRotation (Variables|Default|GetTargetMesh)) false false)))